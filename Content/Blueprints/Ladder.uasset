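; Climbable ladder actor whose height is set by LadderHeigh, with the construction script stacking instanced segments, placing the top and resizing the trigger box.
; While the locally controlled player is in the box, Tick starts climbing on the custom movement component when they move and face along the Arrow, jumping first if grounded.
; During climbing, a 2D cross product against the Arrow nudges the player sideways toward the centre.
; Leaving the box ends the climb.
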(event OnComponentBeginOverlap(Box)
  (params (OverlappedComponent :type Primitive%20Component%20Object%20Reference) (OtherActor :type Actor%20Object%20Reference) (OtherComp :type Primitive%20Component%20Object%20Reference) (OtherBodyIndex :type Integer) (bFromSweep :type Boolean) (SweepResult :type Hit%20Result%20Structure%20%28by%20ref%29))
  (bind _asbp_player_character (Utilities|Casting|CastToBP_PlayerCharacter OtherActor))
  (if (Pawn|IsLocallyControlled _asbp_player_character)
    (Variables|Default|SetPlayer%20In%20Ladder true)))

(event OnComponentEndOverlap(Box)
  (params (OverlappedComponent :type Primitive%20Component%20Object%20Reference) (OtherActor :type Actor%20Object%20Reference) (OtherComp :type Primitive%20Component%20Object%20Reference) (OtherBodyIndex :type Integer))
  (bind _asbp_player_character (Utilities|Casting|CastToBP_PlayerCharacter OtherActor))
  (if (Pawn|IsLocallyControlled _asbp_player_character)
    (Variables|Default|SetPlayer%20In%20Ladder false)
    (Class|HeartdoomCharacterMovementComponent|ClimbEnd (Variables|/Script/Hexshot.HeartdoomCharacter|GetHeartdoomCharacterMovementComponent _asbp_player_character))))

(event EventBeginPlay)

(event Collision|EventActorBeginOverlap
  (params (OtherActor :type Actor%20Object%20Reference)))

(event EventTick
  (params (DeltaSeconds :type Float%20%28single-precision%29))
  (bind _returnvalue (Utilities|Time|GetWorldDeltaSeconds))
  (bind _returnvalue_2 (Game|GetPlayerCharacter 0))
  (bind _returnvalue_3 (Game|GetPlayerCharacter 0))
  (bind _arrow (Variables|Default|GetArrow))
  (bind _arrow_2 (Variables|Default|GetArrow))
  (bind _arrow_3 (Variables|Default|GetArrow))
  (bind _arrow_4 (Variables|Default|GetArrow))
  (bind _returnvalue_4 (Math|Vector|GetForwardVector _arrow))
  (bind _returnvalue_5 (Transformation|GetActorRotation _returnvalue_3))
  (bind _returnvalue_6 (Math|Vector|GetForwardVector _arrow_3))
  (bind _returnvalue_7 (Transformation|GetWorldLocation _arrow_2))
  (bind _returnvalue_8 (Math|Vector|GetForwardVector _arrow_2))
  (bind _returnvalue_9 (* _returnvalue 25.0))
  (bind _charactermovement (Variables|/Script/Engine.Character|GetCharacterMovement _returnvalue_2))
  (bind (_x _y) (Math|Vector|BreakVector _returnvalue_7))
  (bind _returnvalue_10 (Math|Float|MakeLiteralFloat _returnvalue_9))
  (bind _returnvalue_11 (Pawn|Components|CharacterMovement|GetCurrentAcceleration _charactermovement))
  (bind _returnvalue_12 (Math|Rotator|GetRotationXVector _returnvalue_5))
  (bind _returnvalue_13 (Class|KismetMathLibrary|VectorNormal2D _returnvalue_11 0.0001))
  (bind _returnvalue_14 (Math|Vector|Normalize _returnvalue_12))
  (bind _returnvalue_15 (Math|Vector|DotProduct _returnvalue_13 _returnvalue_4))
  (bind _returnvalue_16 (Math|Vector|DotProduct _returnvalue_14 _returnvalue_6))
  (bind _returnvalue_17 (> _returnvalue_16 0.75))
  (bind _returnvalue_18 (> _returnvalue_15 0.75))
  (bind _returnvalue_19 (and _returnvalue_18 _returnvalue_17))
  (if (Variables|Default|GetPlayer%20In%20Ladder)
    (bind _asbp_player_character (Utilities|Casting|CastToBP_PlayerCharacter (Game|GetPlayerCharacter 0)))
    (if (not (Class|AnimInstance|IsAnyMontagePlaying (Components|SkeletalMesh|GetAnimInstance (Variables|/Script/Engine.Character|GetMesh _asbp_player_character))))
      (if (Class|HeartdoomCharacterMovementComponent|IsClimbing (Variables|/Script/Hexshot.HeartdoomCharacter|GetHeartdoomCharacterMovementComponent _asbp_player_character))
        (if (> (Math|Vector|Distance2D(Vector) (Transformation|GetActorLocation _asbp_player_character) _returnvalue_7) 18.0)
          (Math|Float|CompareFloat (- (* (- (.Y (Math|Vector|BreakVector (Transformation|GetActorLocation _asbp_player_character))) _y) (.x _returnvalue_8)) (* (.y _returnvalue_8) (- (.X (Math|Vector|BreakVector (Transformation|GetActorLocation _asbp_player_character))) _x))) 0.0
            (:>
              (Pawn|Input|AddMovementInput _asbp_player_character (Math|Vector|GetRightVector (Math|Rotator|MakeRotator (.roll (Transformation|GetActorRotation _asbp_player_character)) 0.0 (.yaw (Transformation|GetActorRotation _asbp_player_character)))) (* _returnvalue_10 -1.0) false))
            (:<
              (Pawn|Input|AddMovementInput _asbp_player_character (Math|Vector|GetRightVector (Math|Rotator|MakeRotator (.roll (Transformation|GetActorRotation _asbp_player_character)) 0.0 (.yaw (Transformation|GetActorRotation _asbp_player_character)))) _returnvalue_10 false))))
        (elif (or (AI|Components|NavMovement|IsFalling (Variables|/Script/Hexshot.HeartdoomCharacter|GetHeartdoomCharacterMovementComponent _asbp_player_character)) (Class|HeartdoomCharacterMovementComponent|IsGliding (Variables|/Script/Hexshot.HeartdoomCharacter|GetHeartdoomCharacterMovementComponent _asbp_player_character)))
          (if (or (and (> (Math|Vector|DotProduct (Class|KismetMathLibrary|VectorNormal2D (Variables|/Script/Engine.MovementComponent|GetVelocity (Variables|/Script/Engine.Character|GetCharacterMovement (Game|GetPlayerCharacter 0))) 0.0001) (Math|Vector|GetForwardVector (Variables|Default|GetArrow))) 0.75) _returnvalue_17) _returnvalue_19)
            (Utilities|FlowControl|DoOnce false :!label _label
              (:Completed
                (if (or (AI|Components|NavMovement|IsFalling (Variables|/Script/Hexshot.HeartdoomCharacter|GetHeartdoomCharacterMovementComponent _asbp_player_character)) (Class|HeartdoomCharacterMovementComponent|IsGliding (Variables|/Script/Hexshot.HeartdoomCharacter|GetHeartdoomCharacterMovementComponent _asbp_player_character)))
                  _
                  (else
                    (Character|Jump _asbp_player_character)
                    (Utilities|FlowControl|Delay 0.1)))
                (Variables|/Script/Engine.MovementComponent|SetVelocity (Variables|/Script/Hexshot.HeartdoomCharacter|GetHeartdoomCharacterMovementComponent _asbp_player_character) (* (Variables|/Script/Engine.MovementComponent|GetVelocity (Variables|/Script/Hexshot.HeartdoomCharacter|GetHeartdoomCharacterMovementComponent _asbp_player_character)) (+ (Math|Vector|GetRightVector _arrow_4) (Math|Vector|GetUpVector _arrow_4))))
                (Class|HeartdoomCharacterMovementComponent|ClimbStart (Variables|/Script/Hexshot.HeartdoomCharacter|GetHeartdoomCharacterMovementComponent _asbp_player_character))
                (goto _label Reset)))
            (else
              (if _returnvalue_19 :!label _label_2
                (goto _label))))
          (else
            (goto _label_2)))))))

(fn ConstructionScript
  (bind _box (Variables|Default|GetBox))
  (bind _ladder_heigh (Variables|Default|GetLadder%20Heigh))
  (bind _box_2 (Variables|Default|GetBox))
  (bind _returnvalue (* _ladder_heigh 5e+01))
  (bind _relativelocation (Variables|/Script/Engine.SceneComponent|GetRelativeLocation _box))
  (bind _boxextent (Variables|/Script/Engine.BoxComponent|GetBoxExtent _box_2))
  (bind _returnvalue_2 (+ _returnvalue 1e+02))
  (Transformation|SetRelativeLocation (Variables|Default|GetLadder_LadderTop) (Math|Vector|MakeVector 0.0 0.0 (- (* (Variables|Default|GetLadder%20Heigh) 1e+02) 1e+02)) false false)
  (for _index (range 1 (Variables|Default|GetLadder%20Heigh))
    (Components|InstancedStaticMesh|AddInstance (Variables|Default|GetInstanced%20Ladder_Loop) (Math|Transform|MakeTransform (Math|Vector|MakeVector 0.0 0.0 (- (* _index 1e+02) 1e+02)) "0, 0, 0" "1.000000,1.000000,1.000000") false))
  (Transformation|SetRelativeLocation _box (Math|Vector|MakeVector (.x _relativelocation) (.y _relativelocation) _returnvalue_2) false false)
  (Components|Box|SetBoxExtent _box_2 (Math|Vector|MakeVector (.x _boxextent) (.y _boxextent) _returnvalue_2) true))