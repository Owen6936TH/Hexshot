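; BP_EnemyAiController is an enemy AI controller that maintains a list of actors currently seen through AI Perception sight.
; Perception updates add a sensed actor uniquely and remove it when sight is lost, substituting its parent actor when valid so child actors register as their owner.
; Tick loops over the list and removes invalid entries.
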(event OnTargetPerceptionUpdated(AIPerception)
  (params (Actor :type Actor%20Object%20Reference) (Stimulus :type AI%20Stimulus%20Structure))
  (bind _returnvalue (Actor|GetParentActor Actor))
  (bind _returnvalue_2 (Utilities|IsValid _returnvalue))
  (bind _returnvalue_3 (select _returnvalue_2 _returnvalue Actor))
  (bind _returnvalue_4 (Class|AIPerceptionSystem|GetSenseClassforStimulus Stimulus))
  (if (== _returnvalue_4 "/Script/AIModule.AISense_Sight")
    (if (.bSuccessfullySensed (Utilities|Struct|BreakAIStimulus Stimulus))
      (Utilities|Array|AddUnique (Variables|Default|GetSight%20Actor) _returnvalue_3)
      (else
        (CallFunction|RemoveSightTargetActor _returnvalue_3)))))

(event EventBeginPlay)

(event EventTick
  (params (DeltaSeconds :type Float%20%28single-precision%29))
  (for _array_element (Variables|Default|GetSight%20Actor)
    (Utilities|IsValid _array_element
      (:Is%20Not%20Valid
        (CallFunction|RemoveSightTargetActor _array_element)))))

(fn ConstructionScript)

(fn RemoveSightTargetActor
  (params (Item :type Actor%20Object%20Reference%20%28by%20ref%29))
  (Utilities|Array|RemoveItem (Variables|Default|GetSight%20Actor) Item)
  (return))