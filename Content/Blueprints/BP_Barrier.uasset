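; A barrier actor that removes its barrier component once all enemies in its EnemyActor list are destroyed.
; BeginPlay counts valid enemies and binds their destroy events, which update the count and a dead/required TextRenderActor display.
; OnInflictDamage replays a timeline driving the dynamic material's opacity.
; The construction script sizes and positions the barrier from width and height variables, and its interaction prompt is disabled.
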(event Custom|OnDestroyed_Event
  (params (DestroyedActor :type Actor%20Object%20Reference))
  (Math|Integer|DecrementInt (Variables|Default|GetEnemy%20Left)
    (:%20%20
      (CallFunction|CheckEnemy))))

(event Custom|Check%20Enemy
  (bind _enemy_actor (Variables|Default|GetEnemy%20Actor))
  (bind _returnvalue (Utilities|Array|Length _enemy_actor))
  (Utilities|FlowControl|Sequence
    (:then_0
      (if (<= (Variables|Default|GetEnemy%20Left) 0)
        (Components|DestroyComponent (Variables|Default|GetBarrier))))
    (:then_1
      (bind _astext_render_actor (Utilities|Casting|CastToTextRenderActor (Variables|Default|GetText%20Count)))
      (Rendering|Components|TextRender|SetText (Variables|/Script/Engine.TextRenderActor|GetTextRender _astext_render_actor) (Utilities|Text|FormatText "{Dead}/{Require}" (- _returnvalue (Variables|Default|GetEnemy%20Left)) _returnvalue)))))

(event EventBeginPlay
  (for _array_element (Variables|Default|GetEnemy%20Actor)
    (Utilities|IsValid _array_element
      (:Is%20Valid
        (Game|AssignOnDestroyed _array_element (delegate Custom|OnDestroyed_Event))
        (Math|Integer|IncrementInt (Variables|Default|GetEnemy%20Left)))))
  (bind _returnvalue (Rendering|Material|CreateDynamicMaterialInstance (Variables|Default|GetBarrier) 0 "/Game/Material/Barrier.Barrier" "None" :!class /Script/Engine.PrimitiveComponent))
  (Variables|Default|SetMaterial _returnvalue)
  (CallFunction|CheckEnemy))

(event Collision|EventActorBeginOverlap
  (params (OtherActor :type Actor%20Object%20Reference)))

(event EventTick
  (params (DeltaSeconds :type Float%20%28single-precision%29)))

(event EventOnInflictDamage
  (params (Attacker :type Pawn%20Object%20Reference))
  (bind _opacity (Timeline|BarrierOpacityTimeline PlayFromStart)
    (:Update
      (Rendering|Material|SetScalarParameterValue (Variables|Default|GetMaterial) "Opacity" _opacity :!class /Script/Engine.MaterialInstanceDynamic))))

(fn ConstructionScript
  (Transformation|SetRelativeTransform (Variables|Default|GetBarrier) (Math|Transform|MakeTransform (Math|Vector|MakeVector 0.0 (* (Variables|Default|GetBarrier%20Width) 5e+01) (* (Variables|Default|GetBarrier%20Heigh) 5e+01)) "90.000000,0.000000,0.000000" (Math|Vector|MakeVector (Variables|Default|GetBarrier%20Heigh) (Variables|Default|GetBarrier%20Width) 1.0)) false false))

(fn GetInteractionPrompt
  (return false "" 0))